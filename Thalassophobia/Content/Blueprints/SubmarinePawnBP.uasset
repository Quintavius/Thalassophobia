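; Player-controlled submarine pawn with thrust, vertical movement, yaw and pitch, plus a speed-reactive spring-arm camera.
; Each tick integrates inputs into clamped speeds with friction, pulls pitch back toward level, then sets rotation and adds movement input.
; Camera gimbal and arm rotate, shift and stretch by lerping over normalized speeds.
; The Diving axis drives yaw and Rotating drives pitch; both angles print on screen every frame.
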(event `self.ReceiveBeginPlay`
  (`self.InitCamera`))

(event `self.ReceiveTick`
  (params (DeltaSeconds :type "Float (single-precision)"))
  (`|ExecutionSequence`
    (:`then_0`
      (bind _targetrotation (`self.ComputeRot` DeltaSeconds))
      (`self.K2_SetActorRotation` _targetrotation)
      (`KismetSystemLibrary.PrintString` (`KismetStringLibrary.Concat_StrStr` "pitch :  " (`KismetStringLibrary.Conv_DoubleToString` (`self.curPitch`))) true true (struct :`G` 0.66 :`B` 1.0 :`A` 1.0) 0.0)
      (`KismetSystemLibrary.PrintString` (`KismetStringLibrary.Concat_StrStr` "yaw :  " (`KismetStringLibrary.Conv_DoubleToString` (`self.curYaw`))) true true (struct :`G` 0.66 :`B` 1.0 :`A` 1.0) 0.0))
    (:`then_1`
      (bind _output_get (set `self.acceleration` (`self.ComputeAcceleration` DeltaSeconds)))
      (`self.AddMovementInput` (`KismetMathLibrary.GetForwardVector` _targetrotation) _output_get))
    (:`then_2`
      (bind _output_get_2 (set `self.dropping` (`self.ComputeDropping` DeltaSeconds)))
      (`self.AddMovementInput` (0.0 0.0 1.0) _output_get_2))
    (:`then_3`
      (`self.UpdateCamera`))))

(event `InputAxis|Diving`
  (params (AxisValue :type "Float (single-precision)"))
  (set `self.yawRatio` (stale `InputAxis|Rotating` AxisValue)))

(event `InputAxis|Dropping`
  (params (AxisValue :type "Float (single-precision)"))
  (set `self.droppingRatio` AxisValue))

(event `InputAxis|Rotating`
  (params (AxisValue :type "Float (single-precision)"))
  (set `self.pitchRatio` (stale `InputAxis|Diving` AxisValue)))

(event `InputAction|Thrust`
  (params (Key :type "Key Structure"))
  (:`Pressed`
    (set `self.accelerationRatio` 1.0))
  (:`Released`
    (set `self.accelerationRatio` 0.0)))

(event `UpdateCamera`
  (bind _pitchmaxspeed (`self.pitchMaxSpeed`))
  (bind _yawmaxspeed (`self.yawMaxSpeed`))
  (bind _startarmlength (`self.startArmLength`))
  (bind _camerayaw (`self.cameraYaw`))
  (bind _camerapitch (`self.cameraPitch`))
  (bind _cameraaccelerationoffset (`self.cameraAccelerationOffset`))
  (bind _droppingmaxspeed (`self.droppingMaxSpeed`))
  (bind _cameradroppingoffset (`self.cameraDroppingOffset`))
  (bind _alpha (`self.InverseLerp` 0.0 (`self.forwardMaxSpeed`) (`self.acceleration`)))
  (`SceneComponent.K2_SetRelativeRotation` (`self.AzimuthGimbal`) (`KismetMathLibrary.MakeRotator` 0.0 0.0 (`KismetMathLibrary.Lerp` (* _camerayaw -1.0) _camerayaw (`self.InverseLerp` (* _yawmaxspeed -1.0) _yawmaxspeed (`self.curYawSpeed`)))) false false)
  (`SceneComponent.K2_SetRelativeRotation` (`self.SpringArm`) (`KismetMathLibrary.MakeRotator` 0.0 (+ (`KismetMathLibrary.Lerp` (* _camerapitch -1.0) _camerapitch (`self.InverseLerp` (* _pitchmaxspeed -1.0) _pitchmaxspeed (`self.curPitchSpeed`))) (`self.startPitchCamera`))) false false)
  (`SceneComponent.K2_SetRelativeLocation` (`self.AzimuthGimbal`) (`KismetMathLibrary.MakeVector` (`KismetMathLibrary.Lerp` 0.0 _cameraaccelerationoffset _alpha) 0.0 (`KismetMathLibrary.Lerp` (* _cameradroppingoffset -1.0) _cameradroppingoffset (`self.InverseLerp` (* _droppingmaxspeed -1.0) _droppingmaxspeed (`self.dropping`)))) false false)
  (set `SpringArmComponent.TargetArmLength` (`KismetMathLibrary.Lerp` _startarmlength (+ _startarmlength _cameraaccelerationoffset) _alpha) (`self.SpringArm`)))

(event `InitCamera`
  (set `self.startPitchCamera` (.pitch (.rotation (`SceneComponent.GetRelativeTransform` (`self.SpringArm`)))))
  (set `self.startArmLength` (`SpringArmComponent.TargetArmLength` (`self.SpringArm`))))

(fn `ComputeRot`
  (params (delta :type "Float (double-precision)"))
  (returns (targetRotation :type "Rotator Structure"))
  (bind _pitchclampedangle (`self.pitchClampedAngle`))
  (bind _output_get (set `self.curYawSpeed` (`self.ComputeYawSpeed` delta)))
  (bind _output_get_2 (set `self.curYaw` (+ _output_get (`self.curYaw`))))
  (bind _output_get_3 (set `self.curPitchSpeed` (+ (`self.ComputePitchSpeed` delta) (* (* (`self.curPitch`) (* (`self.pitchReorientForce`) -1.0)) delta))))
  (bind _output_get_4 (set `self.curPitch` (`KismetMathLibrary.FClamp` (+ _output_get_3 (`self.curPitch`)) (* _pitchclampedangle -1.0) _pitchclampedangle)))
  (return (`KismetMathLibrary.MakeRotator` 0.0 _output_get_4 _output_get_2)))

(fn `UserConstructionScript`)